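; BP_SparGameMode is a game mode for a round-based, last-player-standing match, with much of its flow still stubbed.
; It tracks alive flags and scores in per-player maps; ResetRound revives everyone and increments the alive count, while ResetGame zeroes scores.
; OnPlayerDied flags the player dead and calls EndRound if the count is below two, but never decrements it.
; EndRound only prints a message, and StartRound and OnGameComplete are empty.
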(event Custom|Reset%20Game
  (bind _keys (Utilities|Map|Keys (Variables|Default|GetPlayerScores)))
  (for _array_element _keys
    (Utilities|Map|Add (Variables|Default|GetPlayerScores) _array_element 0)))

(event Custom|Start%20Round)

(event Custom|End%20Round
  ;[0.15 0.15 0.15 0.5] Find Last Player, give them point, then reset
  (Development|PrintString "Round Over!"))

(event Custom|On%20Player%20Died
  (params (Dead%20Player :type Player%20Controller%20Object%20Reference))
  ;[0.15 0.15 0.15 0.5] Check if only 1 player remains
  (Utilities|Map|Add (Variables|Default|GetRegisteredPlayers) Dead%20Player false)
  (if (< (Variables|Default|GetbPlayersRemainingAlive) 2)
    (CallFunction|EndRound)))

(event Custom|On%20Game%20Complete
  ;[0.15 0.15 0.15 0.5] Determine Which Player won
)

(event Custom|Reset%20Round
  (bind _keys (Utilities|Map|Keys (Variables|Default|GetRegisteredPlayers)))
  (for _array_element _keys
    (Utilities|Map|Add (Variables|Default|GetRegisteredPlayers) _array_element true)
    (Math|Integer|IncrementInt (Variables|Default|GetbPlayersRemainingAlive))))

(fn ConstructionScript)