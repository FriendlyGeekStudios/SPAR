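; Firearm weapon for Spar characters that fires projectiles from a limited ammo count, which is filled to max on BeginPlay.
; Attack plays a flipbook fire effect, parked on its last frame until fired, and spawns the projectile at the spawn point.
; The SparCharacter owning the mount point's attach parent becomes instigator.
; A DoOnce reset after a delay limits fire rate; no reload exists here.
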(event EventBeginPlay
  (bind _fireeffectanimation (Variables|Default|GetFireEffectAnimation))
  (Components|Timeline|SetLooping (Variables|Default|GetFireEffectAnimation) false)
  (Class|PaperFlipbookComponent|SetPlaybackPositioninFrames _fireeffectanimation (Class|PaperFlipbookComponent|GetFlipbookLengthinFrames _fireeffectanimation) false)
  (Variables|Default|SetRemainingAmmo (Variables|Default|GetMaxAmmo)))

(event EventAttack
  (Utilities|FlowControl|DoOnce false :!label _label
    (:Completed
      (if (> (Variables|Default|GetRemainingAmmo) 0)
        (Components|Timeline|PlayfromStart (Variables|Default|GetFireEffectAnimation))
        (Game|SpawnActorfromClass (Variables|Default|GetProjectileType) (Transformation|GetWorldTransform (Variables|Default|GetProjectileSpawnLocation)) "Undefined" "MultiplyWithRoot" 0 (.AsBP%20Spar%20Character (Utilities|Casting|CastToBP_SparCharacter (Components|GetOwner (Transformation|GetAttachParent (Variables|Default|GetMountPoint))))))
        (Math|Integer|DecrementInt (Variables|Default|GetRemainingAmmo)
          (:%20%20
            (Utilities|FlowControl|Delay (Variables|Default|GetFireRateCooldownDuration))
            (goto _label Reset)))))))

(fn ConstructionScript)